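; Trigger actor that spawns a one-time batch of random zombies when BP_FirstPersonCharacter overlaps it.
; A DoOnce precedes the character cast, so any first overlapping actor uses up the trigger.
; EnemySpawner loops NumberOfEnemies times, picking one of six zombie classes at a random XY offset around the root, always spawning despite collisions.
; After the loop, it spawns one extra random zombie at the last location.
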(event Custom|EnemySpawner
  (params (SpawnTransform :type Transform) (Number%20Of%20Enemies :type Integer))
  (bind _defaultsceneroot (Variables|Default|GetDefaultSceneRoot))
  (bind _returnvalue (Transformation|GetWorldLocation _defaultsceneroot))
  ;[1 1 1] Spawner
  (for _index (range 0 (- Number%20Of%20Enemies 1))
    (bind _output_get (Variables|Default|SetLocationSpawner (Math|Vector|MakeVector (+ (Math|Random|RandomFloatinRange -1.2e+03 1.2e+03) (.x _returnvalue)) (+ (Math|Random|RandomFloatinRange -1.2e+03 1.2e+03) (.y _returnvalue)) (.z _returnvalue))))
    (switch int (Math|Random|RandomIntegerinRange 0 5)
      (:0
        (Game|SpawnActorfromClass "/Game/_Aryan_Pathak/zombieblueprint/BP_MonsterZombie1.BP_MonsterZombie1_C" (Math|Conversions|ToTransform(Vector) _output_get) "AlwaysSpawn" 0 0))
      (:1
        (Game|SpawnActorfromClass "/Game/_Shubham_Shrey/Zombie/ZombiesBlueprints/BP_MonsterZombie2.BP_MonsterZombie2_C" (Math|Conversions|ToTransform(Vector) _output_get) "AlwaysSpawn" 0 0))
      (:2
        (Game|SpawnActorfromClass "/Game/_Shubham_Shrey/Zombie/ZombiesBlueprints/BP_WarZombie.BP_WarZombie_C" (Math|Conversions|ToTransform(Vector) _output_get) "AlwaysSpawn" 0 0))
      (:3
        (Game|SpawnActorfromClass "/Game/_Shubham_Shrey/Zombie/ZombiesBlueprints/BP_ZombieBoy.BP_ZombieBoy_C" (Math|Conversions|ToTransform(Vector) _output_get) "AlwaysSpawn" 0 0))
      (:4
        (Game|SpawnActorfromClass "/Game/_Shubham_Shrey/Zombie/ZombiesBlueprints/BP_ZombieCop.BP_ZombieCop_C" (Math|Conversions|ToTransform(Vector) _output_get) "AlwaysSpawn" 0 0))
      (:5
        (Game|SpawnActorfromClass "/Game/_Shubham_Shrey/Zombie/ZombiesBlueprints/BP_ZombieGirl.BP_ZombieGirl_C" (Math|Conversions|ToTransform(Vector) _output_get) "AlwaysSpawn" 0 0))))
  (switch int (Math|Random|RandomIntegerinRange 0 5)
    (:0
      (Game|SpawnActorfromClass "/Game/_Aryan_Pathak/zombieblueprint/BP_MonsterZombie1.BP_MonsterZombie1_C" (Math|Conversions|ToTransform(Vector) (Variables|Default|GetLocationSpawner)) "AlwaysSpawn" 0 0))
    (:1
      (Game|SpawnActorfromClass "/Game/_Shubham_Shrey/Zombie/ZombiesBlueprints/BP_MonsterZombie2.BP_MonsterZombie2_C" (Math|Conversions|ToTransform(Vector) (Variables|Default|GetLocationSpawner)) "AlwaysSpawn" 0 0))
    (:2
      (Game|SpawnActorfromClass "/Game/_Shubham_Shrey/Zombie/ZombiesBlueprints/BP_WarZombie.BP_WarZombie_C" (Math|Conversions|ToTransform(Vector) (Variables|Default|GetLocationSpawner)) "AlwaysSpawn" 0 0))
    (:3
      (Game|SpawnActorfromClass "/Game/_Shubham_Shrey/Zombie/ZombiesBlueprints/BP_ZombieBoy.BP_ZombieBoy_C" (Math|Conversions|ToTransform(Vector) (Variables|Default|GetLocationSpawner)) "AlwaysSpawn" 0 0))
    (:4
      (Game|SpawnActorfromClass "/Game/_Shubham_Shrey/Zombie/ZombiesBlueprints/BP_ZombieCop.BP_ZombieCop_C" (Math|Conversions|ToTransform(Vector) (Variables|Default|GetLocationSpawner)) "AlwaysSpawn" 0 0))
    (:5
      (Game|SpawnActorfromClass "/Game/_Shubham_Shrey/Zombie/ZombiesBlueprints/BP_ZombieGirl.BP_ZombieGirl_C" (Math|Conversions|ToTransform(Vector) (Variables|Default|GetLocationSpawner)) "AlwaysSpawn" 0 0))))

(event Collision|EventActorBeginOverlap
  (params (OtherActor :type Actor%20Object%20Reference))
  (Utilities|FlowControl|DoOnce false
    (:Completed
      (Utilities|Casting|CastToBP_FirstPersonCharacter OtherActor)
      (CallFunction|EnemySpawner (Math|Conversions|ToTransform(Vector) (Variables|Default|GetLocationSpawner)) (Variables|Default|GetNumber%20Of%20Enemies)))))

(fn ConstructionScript)