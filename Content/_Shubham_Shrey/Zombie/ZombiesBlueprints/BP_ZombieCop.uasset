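; BP_ZombieCop is a zombie cop enemy for the survival mode that chases and attacks the player.
; An AIMoveTo loop starts on BeginPlay and leads into montage attacks, whose notify applies damage through a sphere overlap; sighting the player sets run speed.
; Point damage drains health with hit reactions until death, which disables collision, randomly drops ammo at a ground trace and notifies Survival_GameMode's death counter.
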(event OnSeePawn(PawnSensing)
  (params (Pawn :type Pawn%20Object%20Reference))
  ;[1 1 1] Run to player when in sight
  (Variables|/Script/Engine.CharacterMovementComponent|SetMaxWalkSpeed (Variables|Character|GetCharacterMovement) 3.6e+02))

(event Custom|RunToPlayer
  ;[1 1 1] Chase Player Logic
  (if (not (Variables|Default|GetIsDead))
    (AI|AIMoveTo self "0, 0, 0" (Game|GetPlayerController 0) 4e+01 false
      (:OnSuccess
        (CallFunction|AttackPlayer))
      (:OnFail
        (CallFunction|RuntoPlayer)))))

(event Custom|Attack%20Player
  ;[1 1 1] Attack Player and Randomize
  (Animation|Montage|PlayMontage (Variables|Character|GetMesh) "/Game/_Shubham_Shrey/Zombie/ZombieCop/Animations/Zombie_Attack_Montage_Cop.Zombie_Attack_Montage_Cop"
    (:OnCompleted
      (CallFunction|RuntoPlayer :!label _label))
    (:OnInterrupted
      (goto _label))
    (:OnNotifyBegin
      (bind _outactors (Actor|GetAllActorswithTag "Enemy"))
      (bind (_outactors_2 _returnvalue) (Collision|SphereOverlapActors (Transformation|GetWorldLocation (Variables|Default|GetArrow1)) 8e+01 (Utilities|Array|MakeArray "ObjectTypeQuery3") "/Game/FirstPerson/Blueprints/BP_FirstPersonCharacter.BP_FirstPersonCharacter_C" _outactors))
      (if _returnvalue
        (for _array_element _outactors_2
          (Game|Damage|ApplyDamage _array_element 2e+01 (Pawn|GetController) self "/Script/Engine.DamageType"))))))

(event Custom|Death
  (bind _returnvalue (Transformation|GetActorLocation))
  ;[1 1 1] Death Event (By _Dev_Verma)
  (Variables|Default|SetIsDead true)
  (Components|Movement|StopMovementImmediately (Variables|Character|GetCharacterMovement))
  (Animation|Montage|PlayMontage (Variables|Character|GetMesh) "/Game/_Shubham_Shrey/Zombie/ZombieCop/Animations/Zombie_Death_Montage_cop.Zombie_Death_Montage_cop"
    (:then
      (Collision|SetCollisionResponsetoChannel (Variables|Collision|GetCapsuleComponent) "ECC_Pawn" "ECR_Overlap")
      (Collision|SetCollisionEnabled (Variables|Character|GetMesh) "NoCollision")
      (Actor|SetLifeSpan self 5.0)
      (if (Math|Random|RandomBoolwithWeight 0.45)
        (bind _outhit (Collision|LineTraceByChannel _returnvalue (- _returnvalue "0,0,1000.000000") "TraceTypeQuery1" false 0 "None"))
        (Game|SpawnActorfromClass "/Game/_Shubham_Shrey/Assests/BP_Ammo.BP_Ammo_C" (Math|Transform|MakeTransform (.Location (Collision|BreakHitResult _outhit)) "0, 0, 0" "1.000000,1.000000,1.000000") "Undefined" 0 0))
      (bind _assurvival_game_mode (Utilities|Casting|CastToSurvival_GameMode (Game|GetGameMode)))
      (Default|DeathCouner _assurvival_game_mode))))

(event EventBeginPlay
  ;[1 1 1] Event BeginPlay
  (CallFunction|RuntoPlayer))

(event Game|Damage|EventPointDamage
  (params (Damage :type Float%20%28single-precision%29) (DamageType :type Damage%20Type%20Object%20Reference) (HitLocation :type Vector :default "0, 0, 0") (HitNormal :type Vector :default "0, 0, 0") (HitComponent :type Primitive%20Component%20Object%20Reference) (BoneName :type Name :default "None") (ShotFromDirection :type Vector :default "0, 0, 0") (InstigatedBy :type Controller%20Object%20Reference) (DamageCauser :type Actor%20Object%20Reference) (HitInfo :type Hit%20Result%20Structure%20%28by%20ref%29))
  ;[1 1 1] Getting Damage System (by _Dev_Verma)
  (if (not (Variables|Default|GetisDead))
    (if (<= (Variables|Default|GetHealth) 0.0)
      (CallFunction|Death)
      (else
        (bind _output_get (Variables|Default|SetHealth (- (Variables|Default|GetHealth) Damage)))
        (if (<= _output_get 0.0)
          (CallFunction|Death)
          (else
            (Animation|Montage|PlayMontage (Variables|Character|GetMesh) "/Game/_Shubham_Shrey/Zombie/ZombieCop/Animations/Zombie_Reaction_Hit_Montage_cop.Zombie_Reaction_Hit_Montage_cop")))))))

(fn ConstructionScript)